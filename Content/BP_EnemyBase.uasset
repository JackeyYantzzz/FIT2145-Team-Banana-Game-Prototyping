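; Base 2D flipbook enemy that follows a spline path and can be killed by damage.
; BeginPlay starts the walk animation, initializes HP and grabs the BP_SplinePath actor returned by GetActorOfClass.
; Tick advances distance by MoveSpeed, matches location and rotation to the spline, and destroys the enemy at its end.
; Lethal damage disables collision, plays the death flipbook and destroys the actor after a short delay, without halting movement.
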(event Custom|TakeDamage
  (params (DamageAmount :type Float%20%28double-precision%29))
  (bind _output_get (Variables|Default|SetCurrentHP (- (Variables|Default|GetCurrentHP) DamageAmount)))
  (if (<= _output_get 0.0)
    (Collision|SetActorEnableCollision false)
    (Sprite|SetFlipbook (Variables|Default|GetEnemySprite) (Variables|Default|GetDeathFlipbook))
    (Utilities|FlowControl|Delay 0.5)
    (Actor|DestroyActor)))

(event EventBeginPlay
  (Sprite|SetFlipbook (Variables|Default|GetEnemySprite) (Variables|Default|GetWalkFlipbook))
  (Variables|Default|SetCurrentHP (Variables|Default|GetMaxHP))
  (bind _returnvalue (Actor|GetActorOfClass "/Game/BP_SplinePath.BP_SplinePath_C"))
  (Variables|Default|SetTargetSpline _returnvalue))

(event Collision|EventActorBeginOverlap
  (params (OtherActor :type Actor%20Object%20Reference)))

(event EventTick
  (params (DeltaSeconds :type Float%20%28single-precision%29))
  (bind _targetspline (Variables|Default|GetTargetSpline))
  (bind _spline (Variables|/Game/BP_SplinePath.BP_SplinePath_C|GetSpline _targetspline))
  (Utilities|IsValid _targetspline
    (:Is%20Valid
      (bind _output_get (Variables|Default|SetDistanceAlongSpline (+ (* DeltaSeconds (Variables|Default|GetMoveSpeed)) (Variables|Default|GetDistanceAlongSpline))))
      (Transformation|SetActorLocationAndRotation (Spline|GetLocationatDistanceAlongSpline _spline _output_get "World") (Spline|GetRotationatDistanceAlongSpline _spline _output_get "World"))
      (if (>= _output_get (Spline|GetSplineLength _spline))
        (Actor|DestroyActor)))))

(fn ConstructionScript)